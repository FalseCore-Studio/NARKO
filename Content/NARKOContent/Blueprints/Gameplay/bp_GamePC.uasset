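; Gameplay player controller that sets up the main HUD and handles a debug-printed friend list key.
; BeginPlay hides the mouse cursor, switches to game-only input and creates the gameplay UI widget on the viewport.
; P is meant to toggle the friend list, but branches on reference validity rather than visibility: valid removes it, invalid calls AddToViewport on the empty reference.
; Nothing here creates or assigns that friend list reference.
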(event EventBeginPlay
  (Variables|Default|SetbShowMouseCursor false)
  (Input|SetInputModeGameOnly self)
  (bind _returnvalue (UserInterface|CreateWidget "/Game/NARKOContent/Blueprints/Gameplay/ui_GameplayUI.ui_GameplayUI_C"))
  (bind _output_get (Variables|Default|Setv_MainUIRef _returnvalue))
  (UserInterface|Viewport|AddtoViewport _output_get 0))

(event Input|KeyboardEvents|P
  (params (Key :type Key%20Structure :default "None"))
  (bind _friendlistref (Variables|Default|GetFriendListRef))
  (:Pressed
    (Utilities|IsValid (Variables|Default|GetFriendListRef)
      (:Is%20Valid
        (Widget|RemovefromParent _friendlistref)
        (Development|PrintString "Remove"))
      (:Is%20Not%20Valid
        (UserInterface|Viewport|AddtoViewport _friendlistref 0)
        (Development|PrintString "Add")))))

(fn ConstructionScript)