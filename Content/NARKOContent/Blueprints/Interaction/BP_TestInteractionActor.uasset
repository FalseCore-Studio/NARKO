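; Test interactable actor with a cube and a point light that interaction switches on and off.
; Interface focus toggles the cube's custom depth render, and a getter exposes its interaction widget.
; Interact calls InteractOnServer, which flips the RepNotify InteractToggle, whose OnRep sets the light's visibility to keep it in sync across the network.
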(event Custom|InteractOnServer
  ;[1 1 1 1 15] Create 15.04.2025 "PointLight" |Class Defaults - Replicates(True) and Always Relevant(True)
  (Variables|Default|SetInteractToggle (not (Variables|Default|GetInteractToggle))))

(event EventBeginPlay)

(event Collision|EventActorBeginOverlap
  (params (OtherActor :type Actor%20Object%20Reference)))

(event EventTick
  (params (DeltaSeconds :type Float%20%28single-precision%29)))

(event EventInterfaceInteract
  ;[1 1 1 1 15] Create 15.04.2025 "PointLight" |Class Defaults - Replicates(True) and Always Relevant(True)
  (CallFunction|InteractonServer))

(event EventInterfaceToggleFocus
  (params (Focus :type Boolean))
  (Rendering|SetRenderCustomDepth (Variables|Components|GetCube) Focus))

(fn ConstructionScript)

(fn OnRepInteractToggle
  (bind _pointlight (Variables|Default|GetPointLight))
  ;[1 1 1] Create 15.04.2025 "PointLight"
  (if (Variables|Default|GetInteractToggle)
    (Rendering|SetVisibility _pointlight true false)
    (else
      (Rendering|SetVisibility _pointlight false false))))

(fn GetInteractionWidgetRef
  (return (Variables|Components|GetWidget)))